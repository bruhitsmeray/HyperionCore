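; Hyperion controller Blueprint that relays chat messages between controllers and into the chat window UI.
; GetChatMessage stores the sender and message, then calls UpdateChat on every BP_HyperionController found in the world.
; UpdateChat passes both values to UpdateWindow on every HyperionUI_ChatWindow widget it finds.
; The construction script and the SenderAuthority OnRep function are empty.
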(event `GetChatMessage`
  (params (Sender :type String) (Message :type Text))
  (`|ExecutionSequence`
    (:`then_0`
      (set `self.SenderMessage` Message)
      (set `self.SenderName` Sender))
    (:`then_1`
      (bind _outactors (`GameplayStatics.GetAllActorsOfClass` "BP_HyperionController_C"))
      (for _array_element _outactors
        (`self.UpdateChat` _array_element (`self.SenderName`) (`self.SenderMessage`))))))

(event `UpdateChat`
  (params (Sender :type String) (Message :type Text))
  (bind _foundwidgets (`WidgetBlueprintLibrary.GetAllWidgetsOfClass` "/HyperionUI/Widgets/Chat/HyperionUI_ChatWindow.HyperionUI_ChatWindow_C" false))
  (for _array_element _foundwidgets
    (`/HyperionUI/Widgets/Chat/HyperionUI_ChatWindow.UpdateWindow` _array_element Sender Message)))

(fn `OnRep_SenderAuthority`)

(fn `UserConstructionScript`)