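; BP_BaseWeapon is a base weapon actor that fires the first-person template projectile.
; FireWeapon spawns a FirstPersonProjectile at the Sphere component's location plus GunOffset rotated by the player camera, facing the camera's rotation, then plays a fire sound at the actor.
; The construction script tints the gun mesh by writing GunColor into its BodyColor material parameter.
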(event `self.ReceiveTick`
  (params (DeltaSeconds :type "Float (single-precision)")))

(event `FireWeapon`
  (bind _returnvalue (`SceneComponent.K2_GetComponentRotation` (`PlayerCameraManager.TransformComponent` (`GameplayStatics.GetPlayerCameraManager` 0))))
  (`|SpawnActorFromClass` "/HyperionCore/External/FPWeapon/Blueprints/FirstPersonProjectile.FirstPersonProjectile_C" (`KismetMathLibrary.MakeTransform` (+ (`SceneComponent.K2_GetComponentLocation` (`self.Sphere`)) (`KismetMathLibrary.GreaterGreater_VectorRotator` (`self.GunOffset`) _returnvalue)) _returnvalue) "Undefined" "OverrideRootScale" null null)
  (`GameplayStatics.PlaySoundAtLocation` "/HyperionCore/External/FirstPerson/Audio/FirstPersonTemplateWeaponFire02.FirstPersonTemplateWeaponFire02" (`self.K2_GetActorLocation`) (struct) 1.0 1.0 0.0 null null null))

(fn `UserConstructionScript`
  (`MeshComponent.SetVectorParameterValueOnMaterials` (`self.GunMesh`) "BodyColor" (`KismetMathLibrary.Conv_LinearColorToVector` (`self.GunColor`))))