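; Base Hyperion character Blueprint that handles crouch input, with an optional smooth crouch in place of the built-in Crouch and UnCrouch.
; Smooth crouch drives capsule half-height through a timeline and swaps walk speed for crouch speed.
; Releasing crouch reverses the timeline only if a capsule trace finds no obstruction; a blocked release leaves the character crouched.
; BeginPlay passes the last confirmed screen resolution to SetDrawSizeByScreenResolution.
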(event `BeginCrouch`
  ;[1 1 1] Custom Events
  (if (`self.bUseSmoothCrouch`)
    (set `self.bIsCrouching` true)
    (set `CharacterMovementComponent.MaxWalkSpeed` (`self.BaseCrouchSpeed`) (`self.CharacterMovement`))
    (bind (_direction _alpha) (`Timeline|Timeline_1` :!label _label)
      (:`Update`
        (`CapsuleComponent.SetCapsuleHalfHeight` (`self.CapsuleComponent`) (`KismetMathLibrary.Lerp` 90.0 45.0 _alpha) true)))
    (else
      (`self.Crouch`))))

(event `StopCrouch`
  (bind _returnvalue (`SceneComponent.K2_GetComponentLocation` (`self.CapsuleComponent`)))
  ;[1 1 1] Custom Events
  (if (`self.bUseSmoothCrouch`)
    (bind (_outhit _returnvalue_2) (`KismetSystemLibrary.CapsuleTraceSingle` (+ _returnvalue (0.0 0.0 45.0)) (+ _returnvalue (0.0 0.0 90.0)) 34.0 90.0 "TraceTypeQuery1" true))
    (if (not _returnvalue_2)
      (set `self.bIsCrouching` false)
      (set `CharacterMovementComponent.MaxWalkSpeed` (`self.BaseWalkSpeed`) (`self.CharacterMovement`))
      (goto _label :!via `Reverse`))
    (else
      (`self.UnCrouch`))))

(event `InputAction|Crouch`
  (params (Key :type "Key Structure"))
  (:`Pressed`
    (`self.BeginCrouch`))
  (:`Released`
    (`self.StopCrouch`)))

(event `self.ReceiveBeginPlay`
  (bind _returnvalue (`GameUserSettings.GetGameUserSettings`))
  (`self.SetDrawSizeByScreenResolution` (`KismetMathLibrary.Conv_IntPointToVector2D` (`GameUserSettings.GetLastConfirmedScreenResolution` _returnvalue))))

(fn `UserConstructionScript`)