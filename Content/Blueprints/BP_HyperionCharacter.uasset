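; Player character Blueprint that adds smooth crouching, camera zoom and sprint input handling.
; Smooth crouch, when enabled, animates capsule half height on a timeline and slows walk speed, otherwise using standard Crouch.
; Uncrouching runs a capsule trace for headroom before reversing the timeline and restoring the saved walk speed.
; Zoom plays a timeline through the PlayZoom macro to narrow camera FOV, while sprint calls BeginSprint and StopSprint.
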(event `SmoothCrouch`
  ;[1 1 1] Smooth Crouch
  (if (`self.bUseSmoothCrouch`)
    (`|ExecutionSequence`
      (:`then_0`
        (bind _returnvalue (`self.UpdateLastKnownWalkSpeed`)))
      (:`then_1`
        (set `self.bIsCrouching` true)
        (set `CharacterMovementComponent.MaxWalkSpeed` (/ _returnvalue 1.5) (`self.CharacterMovement`))
        (bind (_direction _alpha) (`Timeline|A_SmoothCrouch` :!label _label)
          (:`Update`
            (`CapsuleComponent.SetCapsuleHalfHeight` (`self.CapsuleComponent`) (`KismetMathLibrary.Lerp` 90.0 45.0 _alpha) true)))))
    (else
      (`self.Crouch`))))

(event `SmoothUnCrouch`
  (bind _returnvalue (`SceneComponent.K2_GetComponentLocation` (`self.CapsuleComponent`)))
  ;[1 1 1] Smooth Crouch
  (if (`self.bUseSmoothCrouch`)
    (bind (_outhit _returnvalue_2) (`KismetSystemLibrary.CapsuleTraceSingle` (+ _returnvalue (0.0 0.0 45.0)) (+ _returnvalue (0.0 0.0 90.0)) 34.0 90.0 "TraceTypeQuery1"))
    (if (not _returnvalue_2)
      (set `self.bIsCrouching` false)
      (set `CharacterMovementComponent.MaxWalkSpeed` (`self.LastKnownMovSpeed`) (`self.CharacterMovement`))
      (goto _label :!via `Reverse`))
    (else
      (`self.UnCrouch`))))

(event `InputAction|Crouch`
  (params (Key :type "Key Structure"))
  (:`Pressed`
    (`self.SmoothCrouch`))
  (:`Released`
    (`self.SmoothUnCrouch`)))

(event `InputAction|Zoom`
  (params (Key :type "Key Structure"))
  (bind _basefov (`self.BaseFoV`))
  (:`Pressed`
    (bind (_direction _alpha) (`Timeline|A_Zoom` :!label _label_2)
      (:`Update`
        (`CameraComponent.SetFieldOfView` (`self.Camera`) (`KismetMathLibrary.Lerp` _basefov (/ _basefov 1.5) _alpha)))))
  (:`Released`
    (goto _label_2 :!via `Reverse`)))

(event `InputAction|Sprint`
  (params (Key :type "Key Structure"))
  (:`Pressed`
    (`self.BeginSprint`))
  (:`Released`
    (`self.StopSprint`)))

(fn `UpdateLastKnownWalkSpeed`
  (returns (ReturnValue :type "Float (double-precision)"))
  (if (`NavMovementComponent.IsMovingOnGround` (`self.CharacterMovement`))
    (bind _output_get (set `self.LastKnownMovSpeed` (`CharacterMovementComponent.MaxWalkSpeed` (`self.CharacterMovement`))))
    (return _output_get)))

(fn `UserConstructionScript`)